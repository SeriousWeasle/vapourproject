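; Bullet is a projectile actor whose mesh, speed, damage, gravity, light and effect references come from the BulletList data table, looked up by BulletID in the construction script.
; On overlap it stops moving, and an Identify Actor macro uses casts to sort player, world and enemy hits.
; Only enemies react, losing Health and running CheckHealth.
; The effects are stored but never spawned here, and the bullet self-destructs after a fixed delay.
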(event `self.ReceiveBeginPlay`
  (`KismetSystemLibrary.Delay` 5.0)
  (`self.K2_DestroyActor`))

(event `self.ReceiveActorBeginOverlap`
  (params (OtherActor :type "Actor Object Reference"))
  (`ProjectileMovementComponent.SetVelocityInLocalSpace` (`self.ProjectileMovement`) (0.0 0.0 0.0))
  (bind (_worldactor _playeractor _enemyactor) (`self.Identify Actor` OtherActor)
    (:`Player`
      ;[1 1 1] Comment
      (if (`self.IsFriendly`)
        _))
    (:`Enemy`
      ;[1 1 1] Comment
      (set `/Game/Blueprints/Enemies/EnemyBaseBluePrint.Health` (- (`/Game/Blueprints/Enemies/EnemyBaseBluePrint.Health` _enemyactor) (`self.Damage`)) _enemyactor)
      (`/Game/Blueprints/Enemies/EnemyBaseBluePrint.Check health` _enemyactor))))

(fn `UserConstructionScript`
  (bind _pointlight (`self.PointLight`))
  (bind _returnvalue (`|GetDataTableRow` "/Game/Blueprints/Bullets/BulletList.BulletList" (`KismetStringLibrary.Conv_StringToName` (`KismetStringLibrary.Conv_IntToString` (`self.BulletID`))))
    (:`then`
      (bind (_bulletname _bulletid _damage _speed _mesh _muzzleflash _trail _hitwall _hitenemy _bulletgravity_ _lightrgb _lightintensity) (break `/Game/Blueprints/Bullets/BulletProperties` _returnvalue))
      (`StaticMeshComponent.SetStaticMesh` (`self.BulletMesh`) _mesh)
      (set `ProjectileMovementComponent.InitialSpeed` _speed (`self.ProjectileMovement`))
      (set `self.MuzzleFlash` _muzzleflash)
      (set `self.Trail` _trail)
      (set `self.HitWall` _hitwall)
      (set `self.HitEnemy` _hitenemy)
      (if _bulletgravity_
        (set `ProjectileMovementComponent.ProjectileGravityScale` (`self.GravityScale`) (`self.ProjectileMovement`))
        (else
          (set `ProjectileMovementComponent.ProjectileGravityScale` 0.0 (`self.ProjectileMovement`))))
      (`LightComponent.SetLightColor` _pointlight (`KismetMathLibrary.Conv_ColorToLinearColor` _lightrgb) true)
      (`LightComponent.SetIntensity` _pointlight _lightintensity)
      (set `self.Damage` _damage))
    (:`RowNotFound`
      (`KismetSystemLibrary.PrintString` "Bullet not found"))))